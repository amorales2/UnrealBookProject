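; MyNewHUD is a HUD Blueprint that draws a crosshair and a text label on screen.
; DrawHUD positions both from the screen size, with a small green-tinted Crosshair texture anchored by its top-left corner at the screen midpoint.
; A large black placeholder "TEXT" string in MyFont is drawn at a quarter of the screen width and height.
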(event EventDrawHUD
  (params (SizeX :type Integer) (SizeY :type Integer))
  (Utilities|FlowControl|Sequence
    (:then_0
      (Canvas|DrawTexture "/Game/Textures/crosshair.crosshair" (Math|Conversions|ToFloat(Integer) (/ SizeX 2)) (Math|Conversions|ToFloat(Integer) (/ SizeY 2)) 16.0 16.0 0.0 0.0 1.0 1.0 (Utilities|Struct|MakeLinearColor 0.1 0.8 0.46 1.0)))
    (:then_1
      (HUD|DrawText "TEXT" "(R=0.000000,G=0.000000,B=0.000000,A=1.000000)" (Math|Conversions|ToFloat(Integer) (/ SizeX 4)) (Math|Conversions|ToFloat(Integer) (/ SizeY 4)) "/Game/Textures/MyFont.MyFont" 1e+01 false))))

(fn ConstructionScript)