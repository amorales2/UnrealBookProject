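; BallSpawner is an actor that keeps at most one active Ball, spawned at its own location.
; SpawnBall does nothing while a ball is active; otherwise it spawns one, binds to its overlap event and sets IsSpawnActive.
; When player pawn 0 overlaps the ball, it destroys the ball and clears the flag, allowing the next SpawnBall call to spawn again.
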(event Custom|Spawn%20Ball
  (if (not (Variables|Default|GetIs%20Spawn%20Active))
    (bind _returnvalue (Game|SpawnActorfromClass "/Game/Blueprints/Ball.Ball_C" (Math|Transform|MakeTransform (Transformation|GetActorLocation)) false 0))
    (EventDispatchers|AssignOnActorBeginOverlap _returnvalue (delegate Custom|OverlapBall))
    (Variables|Default|SetIs%20Spawn%20Active true)))

(event Custom|OverlapBall
  (params (OtherActor :type Actor%20Object%20Reference))
  (if (== OtherActor (Game|Player|GetPlayerPawn 0))
    (Actor|DestroyActor (stale Custom|Spawn%20Ball _returnvalue))
    (Variables|Default|SetIs%20Spawn%20Active false)))

(fn ConstructionScript)